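; BP_Sphere is a sphere actor that exercises runtime compositing of tinted texture layers into a render target.
; The construction script puts an M_Test dynamic material instance on the mesh, and BeginPlay composites two scar layers into its base colour parameter.
; A timeline animates the first layer's tint, then swaps that layer to soft smoke and, after a delay, restores the original layers and tints.
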(event `self.ReceiveActorBeginOverlap`
  (params (OtherActor :type "Actor Object Reference")))

(event `self.ReceiveTick`
  (params (DeltaSeconds :type "Float (single-precision)")))

(event `self.ReceiveBeginPlay`
  (bind _returnvalue (`TextureMergeBPLibrary.CreateWithTints` (`|MakeArray` "/Game/Scars1.Scars1" "/Game/Scars2.Scars2" :!type "Texture2D Object Reference") (`|MakeArray` (make `Color` 0 0 255 255) (make `Color` 0 0 255 255))))
  (bind _output_get (set `self.CompositeTexture` _returnvalue))
  (`MaterialInstanceDynamic.SetTextureParameterValue` (`self.MaterialInstance`) "BaseColorParam2D" _output_get)
  (bind (_direction _newtrack_1) (`Timeline|Timeline_0` :!via `PlayFromStart`)
    (:`Update`
      (`TextureMergeBPLibrary.UpdateTint` (`self.CompositeTexture`) (`KismetMathLibrary.Conv_LinearColorToColor` _newtrack_1)))
    (:`Finished`
      (`TextureMergeBPLibrary.UpdateLayer` (`self.CompositeTexture`) "/Engine/Tutorial/SubEditors/TutorialAssets/T_soft_smoke.T_soft_smoke")
      (`KismetSystemLibrary.Delay` 3.0)
      (`TextureMergeBPLibrary.UpdateAllLayers` (`self.CompositeTexture`) (`|MakeArray` "/Game/Scars1.Scars1" "/Game/Scars2.Scars2" :!type "Texture2D Object Reference"))
      (`TextureMergeBPLibrary.UpdateAllTints` (`self.CompositeTexture`) (`|MakeArray` (make `Color` 0 0 255 255) (make `Color` 0 0 255 255))))))

(fn `UserConstructionScript`
  (bind _returnvalue (`KismetMaterialLibrary.CreateDynamicMaterialInstance` "/Game/M_Test.M_Test"))
  (set `self.MaterialInstance` _returnvalue)
  (`PrimitiveComponent.SetMaterial` (`self.StaticMesh`) 0 (`self.MaterialInstance`)))